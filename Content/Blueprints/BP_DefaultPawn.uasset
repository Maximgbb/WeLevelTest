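; Default pawn that lets the player toggle a bool on the level's BP_TargetActor.
; BeginPlay adds the IMC_Default Enhanced Input mapping for player controller 0 and shows the WBP_Hint widget.
; The IA_ToggleBool input calls a server-named event, which finds the target through GetActorOfClass and calls its ToogleBool.
; A controller cast leading into the setup is left unconnected.
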(event Custom|Server_ToggleBoolValue
  (bind _returnvalue (Actor|GetActorOfClass "/Game/Blueprints/BP_TargetActor.BP_TargetActor_C"))
  (Class|TargetActor|ToogleBool _returnvalue))

(event Input|EnhancedActionEvents|EnhancedInputActionIA_ToggleBool
  (params (ActionValue :type Boolean) (ElapsedSeconds :type Float%20%28double-precision%29) (TriggeredSeconds :type Float%20%28double-precision%29) (InputAction :type Input%20Action%20Object%20Reference :default "/Game/Input/Actions/IA_ToggleBool.IA_ToggleBool"))
  (:Started
    (CallFunction|ServerToggleBoolValue)))

(event EventBeginPlay
  (bind _returnvalue (Game|GetPlayerController 0))
  (bind _returnvalue_2 (PlayerController|LocalPlayerSubsystems|GetEnhancedInputLocalPlayerSubsystem _returnvalue))
  (Utilities|IsValid _returnvalue_2
    (:Is%20Valid
      (Input|AddMappingContext _returnvalue_2 "/Game/Input/IMC_Default.IMC_Default" 0 "(bIgnoreAllPressedKeysUntilRelease=True,bForceImmediately=False,bNotifyUserSettings=False)")
      (bind _returnvalue_3 (UserInterface|CreateWidget "/Game/Blueprints/WBP_Hint.WBP_Hint_C" (Game|GetPlayerController 0)))
      (UserInterface|Viewport|AddtoViewport _returnvalue_3 0))))

(fn ConstructionScript)